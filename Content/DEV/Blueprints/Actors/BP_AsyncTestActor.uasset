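; Dev test actor for async loading of static and skeletal mesh parts through a HardData object.
; Events request async part loads, trigger one random mesh swap, or start looping swap timers; OnUnload only prints.
; The load functions set random available parts on AsyncStaticMesh and AsyncSkeletalMesh, printing a warning when data is missing.
; The validity check and mesh assignment roll separate random indices, so they can pick different parts.
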(event `PartInterface.OnUnload`
  (`KismetSystemLibrary.PrintString` "Unload"))

(event `PartInterface.OnTryAsyncLoad_Static`
  (`KismetSystemLibrary.PrintString` "Try Load Async Static")
  (`AL_PartData.RequestAsyncLoad_StaticPart` (`self.HardData`) self))

(event `PartInterface.OnTryAsyncLoad_Skeletal`
  (`KismetSystemLibrary.PrintString` "Try Load Async Skeletal")
  (`AL_PartData.RequestAsyncLoad_SkeletalPart` (`self.HardData`) self))

(event `PartInterface.OnRandomLoad_Static`
  (`KismetSystemLibrary.PrintString` "Random Load Single Static")
  (`self.LoadStaticMeshes`))

(event `PartInterface.OnRandomLoad_Skeletal`
  (`KismetSystemLibrary.PrintString` "Random Load Single Skeletal")
  (`self.LoadSkeletalMeshes`))

(event `PartInterface.OnLoopRandomLoad_Static`
  (`KismetSystemLibrary.PrintString` "Loop Random Load Single Static")
  (bind _returnvalue (`KismetSystemLibrary.K2_SetTimer` null "LoadStaticMeshes" 2.0 true))
  (set `self.StaticLoopLoadHandle` _returnvalue))

(event `PartInterface.OnLoopRandomLoad_Skeletal`
  (`KismetSystemLibrary.PrintString` "Loop Random Load Single Skeletal")
  (bind _returnvalue (`KismetSystemLibrary.K2_SetTimer` null "LoadSkeletalMeshes" 2.0 true))
  (set `self.SkeletalLoopLoadHandle` _returnvalue))

(fn `LoadSkeletalMeshes`
  (bind _asyncskeletalmesh (`self.AsyncSkeletalMesh`))
  (bind _returnvalue (`AL_PartData.GetAvailableSkeletalParts` (`self.HardData`)))
  (bind _skeletalmesh (`SkinnedMeshComponent.SkeletalMesh` (`|GetArrayItem` _returnvalue (`KismetMathLibrary.RandomIntegerInRange` 0 (- (`KismetArrayLibrary.Array_Length` _returnvalue) 1)))))
  (if (> (`KismetArrayLibrary.Array_Length` _returnvalue) 0)
    (`/Engine/EditorBlueprintResources/StandardMacros.IsValid` _asyncskeletalmesh
      (:`Is Valid`
        (`/Engine/EditorBlueprintResources/StandardMacros.IsValid` _skeletalmesh
          (:`Is Valid`
            (`SkinnedMeshComponent.SetSkinnedAssetAndUpdate` _asyncskeletalmesh _skeletalmesh true))
          (:`Is Not Valid`
            (`KismetSystemLibrary.PrintString` "We have not loaded the SKELETAL DATA" :!label _label)))))
    (else
      (goto _label))))

(fn `LoadStaticMeshes`
  (bind _asyncstaticmesh (`self.AsyncStaticMesh`))
  (bind _returnvalue (`AL_PartData.GetAvailableStaticParts` (`self.HardData`)))
  (bind _staticmesh (`StaticMeshComponent.StaticMesh` (`|GetArrayItem` _returnvalue (`KismetMathLibrary.RandomIntegerInRange` 0 (- (`KismetArrayLibrary.Array_Length` _returnvalue) 1)))))
  (if (> (`KismetArrayLibrary.Array_Length` _returnvalue) 0)
    (`/Engine/EditorBlueprintResources/StandardMacros.IsValid` _asyncstaticmesh
      (:`Is Valid`
        (`/Engine/EditorBlueprintResources/StandardMacros.IsValid` _staticmesh
          (:`Is Valid`
            (`StaticMeshComponent.SetStaticMesh` _asyncstaticmesh _staticmesh))
          (:`Is Not Valid`
            (`KismetSystemLibrary.PrintString` "We Haven't loaded the STATIC  Data" :!label _label)))))
    (else
      (goto _label))))

(fn `UserConstructionScript`)